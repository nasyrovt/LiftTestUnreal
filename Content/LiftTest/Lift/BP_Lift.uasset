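; Elevator actor that carries the main character between three floors, using on-board trigger boxes as floor selectors.
; When the lift is available, the box the character overlaps sets the target to the matching floor trigger's location plus a fixed offset.
; Tick eases the lift toward that target with a delta-scaled lerp, marking it available again once it is within a small tolerance.
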(event EventTick
  (params (DeltaSeconds :type Float%20%28single-precision%29))
  ;[1 1 1] Moves an elevator only if it's available
  (if (Utilities|Operators|EqualEqual (Transformation|GetActorLocation) (Variables|Default|GetTargetPosition) 0.2)
    (Variables|Default|SetbIsAvailable true)
    (Variables|Default|SetbIsMoving false)
    (else
      (Variables|Default|SetbIsAvailable false)
      (Variables|Default|SetbIsMoving true)
      (Transformation|SetActorLocation (Math|Vector|Lerp(Vector) (Transformation|GetActorLocation) (Variables|Default|GetTargetPosition) (* DeltaSeconds (Variables|Default|GetSmoothAmount))) false false))))

(event Collision|EventActorBeginOverlap
  (params (OtherActor :type Actor%20Object%20Reference))
  ;[1 1 1] For on-board triggers
  (bind _asbp_main_character (Utilities|Casting|CastToBP_MainCharacter OtherActor))
  (if (Variables|Default|GetbIsAvailable)
    (if (Collision|IsOverlappingActor (Variables|Default|GetBox) _asbp_main_character :!class /Script/Engine.PrimitiveComponent)
      (CallFunction|SetTargetPosition (+ (Transformation|GetActorLocation (Utilities|Array|Get(acopy) (Variables|Default|GetFloorTrigger_0))) "-600.000000,400.000000,0"))
      (elif (Collision|IsOverlappingActor (Variables|Default|GetBox1) _asbp_main_character :!class /Script/Engine.PrimitiveComponent)
        (CallFunction|SetTargetPosition (+ (Transformation|GetActorLocation (Utilities|Array|Get(acopy) (Variables|Default|GetFloorTrigger_0) 1)) "-600.000000,400.000000,0"))
        (elif (Collision|IsOverlappingActor (Variables|Default|GetBox2) _asbp_main_character :!class /Script/Engine.PrimitiveComponent)
          (CallFunction|SetTargetPosition (+ (Transformation|GetActorLocation (Utilities|Array|Get(acopy) (Variables|Default|GetFloorTrigger_0) 2)) "-600.000000,400.000000,0")))))))

(fn ConstructionScript)

(fn SetTargetPosition
  (params (StagePostion :type Vector))
  (Variables|Default|SetTargetPosition StagePostion))